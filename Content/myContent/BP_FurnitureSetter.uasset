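; BP_FurnitureSetter is a manager that tracks and positions the level's furniture actors, gathered by the "Furniture" tag on BeginPlay.
; TakeFurniture picks a random entry from the pending FurnitureOrder list without removing it.
; MoveFurniture relocates a piece and, on success, shifts it from that list to FurnitureDone, which GetDoneFurniture exposes.
; Despite its name, Rotate90DegreeAwayFrom adds a reference actor's upright-aligned rotation to the target's, with no 90-degree offset.
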(event `self.ReceiveBeginPlay`
  (bind _outactors (`GameplayStatics.GetAllActorsWithTag` "Furniture"))
  (set `self.FurnitureOrder` _outactors))

(fn `GetDoneFurniture`
  (returns (Result :type "Array of Actor Object Reference"))
  (return (`self.FurnitureDone`)))

(fn `MoveFurniture`
  (params (Furniture :type "Actor Object Reference") (Location :type "Vector Structure"))
  (returns (MovedSuccessfully :type Boolean))
  (locals (NextFurniture :type "Actor Object Reference"))
  (bind _nextfurniture (`local.NextFurniture`))
  (set `local.NextFurniture` Furniture)
  (bind (_sweephitresult _returnvalue) (`self.K2_SetActorLocation` Furniture Location false false))
  (if _returnvalue
    (`KismetArrayLibrary.Array_Add` (`self.FurnitureDone`) _nextfurniture)
    (bind _returnvalue_2 (`KismetArrayLibrary.Array_RemoveItem` (`self.FurnitureOrder`) _nextfurniture))
    (return (and _returnvalue_2 _returnvalue))
    (else
      (return false))))

(fn `Rotate90DegreeAwayFrom`
  (params (RotateFrom :type "Actor Object Reference") (RotateObj :type "Actor Object Reference"))
  (`self.K2_SetActorRotation` (`local.RotateObj`) (`KismetMathLibrary.MakeRotator` (+ (.roll (`KismetMathLibrary.MakeRotFromZX` (`KismetMathLibrary.MakeVector` 0.0 0.0 1.0) (`KismetMathLibrary.Conv_RotatorToVector` (`self.K2_GetActorRotation` RotateFrom)))) (.roll (`self.K2_GetActorRotation` RotateObj))) (+ (.pitch (`KismetMathLibrary.MakeRotFromZX` (`KismetMathLibrary.MakeVector` 0.0 0.0 1.0) (`KismetMathLibrary.Conv_RotatorToVector` (`self.K2_GetActorRotation` RotateFrom)))) (.pitch (`self.K2_GetActorRotation` RotateObj))) (+ (.yaw (`KismetMathLibrary.MakeRotFromZX` (`KismetMathLibrary.MakeVector` 0.0 0.0 1.0) (`KismetMathLibrary.Conv_RotatorToVector` (`self.K2_GetActorRotation` RotateFrom)))) (.yaw (`self.K2_GetActorRotation` RotateObj)))) false))

(fn `TakeFurniture`
  (returns (Furniture :type "Actor Object Reference"))
  (bind _furnitureorder (`self.FurnitureOrder`))
  (bind _returnvalue (`KismetArrayLibrary.Array_Length` _furnitureorder))
  (if (> _returnvalue 0)
    (return (`|GetArrayItem` _furnitureorder (`KismetMathLibrary.RandomIntegerInRange` 0 (- _returnvalue 1))))
    (else
      (return null))))

(fn `UserConstructionScript`)